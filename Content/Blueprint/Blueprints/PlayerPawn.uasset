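; Player pawn for a tower-building game that copies, carries and rotates physics blocks and raises the camera with the tower.
; Grab traces under the cursor, spawns a copy of a copyable block, counts it and holds it by physics handle.
; Tick moves it with the mouse in Y/Z, while looping timers adjust roll.
; External events release blocks and ease height upward; a trace below the pawn triggers NoBlocks when empty.
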(event Custom|loop%20clockwise
  (bind _rotspeed (Variables|Default|GetRotSpeed))
  ;[1 1 1] Rotate Block
  (if (Variables|Default|GetRotRight)
    (Variables|Default|SetRot (+ (Variables|Default|GetRot) _rotspeed))
    (else
      (Variables|Default|SetRot (- (Variables|Default|GetRot) _rotspeed)))))

(event Custom|ReleaseBlock
  ;[1 1 1] Let go of Block
  (Development|PrintString "release recieved")
  (bind _asmoveable_block (Utilities|Casting|CastToMoveableBlock (Variables|Default|GetHeldBlock)))
  (if (Utilities|IsValid _asmoveable_block)
    (if (Variables|/Game/Blueprint/Blueprints/Blocks/MoveableBlock.MoveableBlock_C|GetLetGoOfMe _asmoveable_block)
      (Physics|Components|PhysicsHandle|ReleaseComponent (Variables|Default|GetPhysicsHandle)))))

(event Custom|Move%20Camera
  (bind _cameraheight (Variables|Default|GetCameraHeight))
  ;[1 1 1] Change Camera Height to Tower Height
  (if (> (Variables|Default|GetCameraHeight) (.z (Transformation|GetWorldLocation (Variables|Collision|GetCapsuleComponent))))
    (bind _newtrack_0 (Timeline|SmoothUp PlayFromStart)
      (:Update
        (Development|PrintString (Utilities|String|ToString(Float) _cameraheight))
        (if (>= _cameraheight 2.5e+02)
          (Transformation|SetWorldLocation (Variables|Transformation|GetRootComponent) (Math|Vector|MakeVector -1.2e+03 0.0 (Math|Interpolation|Ease "EaseInOut" _newtrack_0 (.z (Transformation|GetWorldLocation (Variables|Collision|GetCapsuleComponent))) (Variables|Default|GetCameraHeight) 2.0)) false false))))))

(event EventTick
  (params (DeltaSeconds :type Float%20%28single-precision%29))
  (bind _returnvalue (Game|GetPlayerController 0))
  (bind _originaldistancetoobject (Variables|Default|GetOriginalDistanceToObject))
  (bind _capsulecomponent (Variables|Collision|GetCapsuleComponent))
  (bind (_worldlocation _worlddirection) (Game|Player|ConvertMouseLocationToWorldSpace _returnvalue))
  (bind _returnvalue_2 (Transformation|GetWorldLocation _capsulecomponent))
  (bind _returnvalue_3 (* _worlddirection _originaldistancetoobject))
  (bind _returnvalue_4 (- (.z _returnvalue_2) 2.5e+02))
  (bind _returnvalue_5 (+ _worldlocation _returnvalue_3))
  ;[1 1 1] Hold Block
  (Class|PhysicsHandleComponent|SetTargetLocationandRotation (Variables|Default|GetPhysicsHandle) (Math|Vector|MakeVector 0.0 (.y _returnvalue_5) (.z _returnvalue_5)) (Math|Rotator|MakeRotator (Variables|Default|GetRot) 0.0 0.0))
  ;[1 1 1] Check if camera is too high
  (bind _returnvalue_6 (Collision|LineTraceByChannel (Math|Vector|MakeVector 0.0 2e+03 _returnvalue_4) (Math|Vector|MakeVector 0.0 -2e+03 _returnvalue_4) "TraceTypeQuery1" false 0 "None"))
  (if (not _returnvalue_6)
    (if (Variables|/Game/Blueprint/Blueprints/BlockCopy.BlockCopy_C|GetCheck%20Finished (Variables|Default|GetBlockCopy))
      _
      (else
        _))
    (Default|NoBlocks (Variables|Default|GetBlockCopy))))

(event Input|ActionEvents|InputActionGrab
  (params (Key :type Key%20Structure :default "None"))
  (bind _returnvalue (Game|GetPlayerController 0))
  (bind _returnvalue_2 (Game|GetPlayerController 0))
  (bind (_worldlocation _worlddirection) (Game|Player|ConvertMouseLocationToWorldSpace _returnvalue))
  (bind (_worldlocation_2 _worlddirection_2) (Game|Player|ConvertMouseLocationToWorldSpace _returnvalue_2))
  (:Pressed
    ;[1 1 1] Grab Block Cursor is On
    (bind (_outhit _returnvalue_3) (Collision|LineTraceByChannel _worldlocation_2 (+ _worldlocation_2 (* _worlddirection_2 (Math|Float|MakeLiteralFloat 1e+05))) "TraceTypeQuery2" true 0 "ForDuration")) ; See if Cursor is Over Block
    (if _returnvalue_3
      (if (not (Utilities|IsValid (Class|PhysicsHandleComponent|GetGrabbedComponent (Variables|Default|GetPhysicsHandle)))) ; Not already holding block
        (bind _asmoveable_block (Utilities|Casting|CastToMoveableBlock (.HitActor (Collision|BreakHitResult _outhit))))
        (if (Variables|/Game/Blueprint/Blueprints/Blocks/MoveableBlock.MoveableBlock_C|GetCanCopy _asmoveable_block)
          (Variables|Default|SetOriginalDistanceToObject (.Distance (Collision|BreakHitResult _outhit)))
          (Variables|Default|SetGrabbedBlock (.HitActor (Collision|BreakHitResult _outhit)))
          (bind _returnvalue_4 (Game|SpawnActorfromClass (Utilities|GetClass (.HitActor (Collision|BreakHitResult _outhit))) (Math|Transform|MakeTransform (Math|Vector|MakeVector 0.0 (.y (+ _worldlocation (* _worlddirection (Variables|Default|GetOriginalDistanceToObject)))) (.z (+ _worldlocation (* _worlddirection (Variables|Default|GetOriginalDistanceToObject))))) (Transformation|GetWorldRotation (Variables|/Script/Engine.Actor|GetRootComponent (.HitActor (Collision|BreakHitResult _outhit)))) (Transformation|GetWorldScale (Variables|/Script/Engine.Actor|GetRootComponent (.HitActor (Collision|BreakHitResult _outhit))))) "Undefined" 0 0))
          (Variables|Default|SetHeldBlock _returnvalue_4)
          (bind _asmoveable_block_2 (Utilities|Casting|CastToMoveableBlock _returnvalue_4))
          (Collision|SetCollisionProfileName (Actor|GetComponentbyClass _returnvalue_4 "/Script/Engine.PrimitiveComponent") "Grabbed" true :!class /Script/Engine.PrimitiveComponent) ; Won't Collide with Traces
          (Variables|/Game/Blueprint/Blueprints/Blocks/MoveableBlock.MoveableBlock_C|SetCanCopy _asmoveable_block_2 false)
          (Variables|Default|SetRot 0.0)
          (Rendering|Material|SetMaterial (Actor|GetComponentbyClass _returnvalue_4 "/Script/Engine.PrimitiveComponent") 0 (Rendering|Material|GetMaterial (.HitComponent (Collision|BreakHitResult _outhit)) 0))
          (Collision|SetCollisionEnabled (Actor|GetComponentbyClass _returnvalue_4 "/Script/Engine.PrimitiveComponent") "QueryAndPhysics")
          (Physics|SetSimulatePhysics (Actor|GetComponentbyClass _returnvalue_4 "/Script/Engine.PrimitiveComponent") true)
          (Rendering|SetCastShadow (Actor|GetComponentbyClass _returnvalue_4 "/Script/Engine.PrimitiveComponent") true)
          (Physics|Components|PhysicsHandle|GrabComponentatLocationwithRotation (Variables|Default|GetPhysicsHandle) (Actor|GetComponentbyClass _returnvalue_4 "/Script/Engine.PrimitiveComponent") "None" (Math|Vector|MakeVector 0.0 (.y (.Location (Collision|BreakHitResult _outhit))) (.z (.Location (Collision|BreakHitResult _outhit)))) "0, 0, 0")
          (bind _astowering_up_game_instance (Utilities|Casting|CastToToweringUpGameInstance (Game|GetGameInstance)))
          (Math|Integer|IncrementInt (Variables|/Game/Blueprint/Blueprints/ToweringUpGameInstance.ToweringUpGameInstance_C|GetBlocks%20Used _astowering_up_game_instance)))))))

(event Input|ActionEvents|InputActionClockwiseRotation
  (params (Key :type Key%20Structure :default "None"))
  ;[1 1 1] Rotate Block
  (:Pressed
    (Variables|Default|SetRotRight true)
    (bind _returnvalue (Utilities|Time|SetTimerbyEvent (delegate Custom|loop%20clockwise) 0.01 true)))
  (:Released
    (Utilities|Time|ClearandInvalidateTimerbyHandle _returnvalue)))

(event Input|ActionEvents|InputActionCounter-ClockwiseRotation
  (params (Key :type Key%20Structure :default "None"))
  ;[1 1 1] Rotate Block
  (:Pressed
    (Variables|Default|SetRotRight false)
    (bind _returnvalue (Utilities|Time|SetTimerbyEvent (delegate Custom|loop%20clockwise) 0.01 true)))
  (:Released
    (Utilities|Time|ClearandInvalidateTimerbyHandle _returnvalue)))

(fn ConstructionScript)