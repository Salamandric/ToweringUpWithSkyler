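; WinBox is a win-zone actor that shows a countdown widget while a tower MoveableBlock overlaps it.
; Every tick it scans overlapping blocks, treating a Visibility collision response that stringifies to "2" as tower membership, and stores a match as KeyBlock.
; A match sets WinGood and adds a reused WinCountdown widget to the viewport.
; When KeyBlock ends overlap, WinGood clears and the widget is removed.
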(event EventTick
  (params (DeltaSeconds :type Float%20%28single-precision%29))
  ;[1 1 1] Check if moveableblock that is part of tower
  (for _array_element (Collision|GetOverlappingActors "/Game/Blueprint/Blueprints/Blocks/MoveableBlock.MoveableBlock_C" :!class /Script/Engine.Actor)
    (Development|PrintString (Utilities|String|ToString(Byte) (Collision|GetCollisionResponsetoChannel (Actor|GetComponentbyClass _array_element "/Script/Engine.PrimitiveComponent") "ECC_Visibility")))
    (if (Utilities|Enum|Equal(Enum) (Utilities|String|ToString(Byte) (Collision|GetCollisionResponsetoChannel (Actor|GetComponentbyClass _array_element "/Script/Engine.PrimitiveComponent") "ECC_Visibility")) "2")
      (Variables|Default|SetWinGood true)
      (Variables|Default|SetKeyBlock _array_element)))
  ;[1 1 1] Add Countdown Bar
  (if (Variables|Default|GetWinGood)
    (Utilities|IsValid (Variables|Default|GetCountdownHUD)
      (:Is%20Valid
        (if (not (UserInterface|Viewport|IsinViewport (Variables|Default|GetCountdownHUD)))
          (UserInterface|Viewport|AddtoViewport (Variables|Default|GetCountdownHUD) 0 :!label _label)))
      (:Is%20Not%20Valid
        (bind _returnvalue (UserInterface|CreateWidget "/Game/Blueprint/Blueprints/UI/WinCountdown.WinCountdown_C"))
        (Variables|Default|SetCountdownHUD _returnvalue)
        (goto _label)))))

(event Collision|EventActorEndOverlap
  (params (OtherActor :type Actor%20Object%20Reference))
  (bind _countdownhud (Variables|Default|GetCountdownHUD))
  ;[1 1 1] Remove Countdown when block stops overlap
  (if (== OtherActor (Variables|Default|GetKeyBlock))
    (Variables|Default|SetWinGood false)
    (Utilities|IsValid _countdownhud
      (:Is%20Valid
        (Widget|RemovefromParent _countdownhud)))))

(fn ConstructionScript)