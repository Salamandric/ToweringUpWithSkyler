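; BlockCopy is a Blueprint that sets the player camera height from the top of the block tower.
; ChangeHeight buffers the Z position of each physics-simulating MoveableBlock flagged as a tower block, then sets the PlayerPawn's CameraHeight a fixed offset above the maximum and calls MoveCamera.
; NoBlocks clears the height arrays and reruns ChangeHeight.
; Sorting and tower-gap checks are present but never run.
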(event Custom|ChangeHeight
  (Variables|Default|SetCheck%20Finished false)
  (bind _outactors (Actor|GetAllActorsOfClass "/Game/Blueprint/Blueprints/Blocks/MoveableBlock.MoveableBlock_C"))
  ;[1 1 1] Get Location of each block
  (for _array_element _outactors
    (if (Physics|IsSimulatingPhysics (Variables|/Script/Engine.Actor|GetRootComponent _array_element) "None")
      (if (Variables|/Game/Blueprint/Blueprints/Blocks/MoveableBlock.MoveableBlock_C|GetIsTowerBlock _array_element)
        (Utilities|Array|Add (Variables|Default|GetBuffer) (.z (Transformation|GetWorldLocation (Variables|/Script/Engine.Actor|GetRootComponent _array_element)))))))
  ;[1 1 1] Set Camera Height to Highest point on tower
  (bind _asplayer_pawn (Utilities|Casting|CastToPlayerPawn (Game|GetPlayerCharacter 0)))
  (bind _output_get (Variables|/Game/Blueprint/Blueprints/PlayerPawn.PlayerPawn_C|SetCameraHeight _asplayer_pawn (+ (.MaxValue (Math|Float|MaxOfFloatArray (Variables|Default|GetBuffer))) 2.5e+02)))
  (Development|PrintString (Utilities|String|ToString(Float) _output_get))
  (Variables|Default|SetCheck%20Finished true)
  (Default|MoveCamera _asplayer_pawn))

(event Custom|NoBlocks
  (Development|PrintString "No Blocks Recieved")
  (Utilities|Array|Clear (Variables|Default|GetBlockHeights))
  (Utilities|Array|Clear (Variables|Default|GetBuffer))
  (CallFunction|ChangeHeight))