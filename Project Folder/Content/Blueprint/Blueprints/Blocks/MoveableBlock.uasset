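; MoveableBlock is a physics block the player carries and drops to become part of a tower.
; Its first hit marks it as a tower block, swaps collision profile, releases it from PlayerPawn's grab and, unless it struck Pegs, updates height through BlockCopy and plays a velocity-driven impact sound.
; Destruction notifies BlockCopy.
; To save physics cost, Tick toggles simulation by vertical distance from the player and destroys distant fallen blocks.
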(event EventTick
  (params (DeltaSeconds :type Float%20%28single-precision%29))
  (bind _block (Variables|Replication|GetBlock))
  ;[1 1 1] Optimize physics
  (if (Variables|Default|GetIsTowerBlock)
    (bind _asplayer_pawn (Utilities|Casting|CastToPlayerPawn (Game|Player|GetPlayerPawn 0)))
    (if (and (> (Math|Float|Absolute(Float) (- (.z (Transformation|GetWorldLocation (Variables|Replication|GetBlock))) (.z (Transformation|GetWorldLocation (Variables|/Script/Engine.Actor|GetRootComponent _asplayer_pawn))))) 1e+03) (Variables|Default|GetFallenBlock))
      (Actor|DestroyActor)
      (elif (> (Math|Float|Absolute(Float) (- (.z (Transformation|GetWorldLocation (Variables|Replication|GetBlock))) (.z (Transformation|GetWorldLocation (Variables|/Script/Engine.Actor|GetRootComponent _asplayer_pawn))))) 1.5e+03)
        (Physics|SetSimulatePhysics _block false)
        (else
          (Physics|SetSimulatePhysics _block true))))))

(event EventDestroyed
  ;[1 1 1] Removes Height when deleted
  (bind _asplayer_pawn (Utilities|Casting|CastToPlayerPawn (Game|GetPlayerCharacter 0)))
  (Default|NoBlocks (Variables|/Game/Blueprint/Blueprints/PlayerPawn.PlayerPawn_C|GetBlockCopy _asplayer_pawn)))

(event Collision|EventHit
  (params (MyComp :type Primitive%20Component%20Object%20Reference) (Other :type Actor%20Object%20Reference) (OtherComp :type Primitive%20Component%20Object%20Reference) (bSelfMoved :type Boolean) (HitLocation :type Vector :default "0, 0, 0") (HitNormal :type Vector :default "0, 0, 0") (NormalImpulse :type Vector :default "0, 0, 0") (Hit :type Hit%20Result%20Structure%20%28by%20ref%29))
  (bind _returnvalue (Transformation|GetVelocity))
  (bind _returnvalue_2 (Math|Vector|VectorLength _returnvalue))
  ;[1 1 1] Release Block when hit
  (if (not (Variables|Default|GetIsTowerBlock))
    (Collision|SetCollisionProfileName (Variables|Replication|GetBlock) (Variables|Default|GetCollision%20Name) true :!class /Script/Engine.PrimitiveComponent)
    (Variables|Default|SetIsTowerBlock true)
    (Variables|Default|SetLetGoOfMe true)
    (bind _asplayer_pawn (Utilities|Casting|CastToPlayerPawn (Game|GetPlayerCharacter 0)))
    (if (== (Class|PhysicsHandleComponent|GetGrabbedComponent (Variables|/Game/Blueprint/Blueprints/PlayerPawn.PlayerPawn_C|GetPhysicsHandle _asplayer_pawn)) (Variables|Replication|GetBlock)) ; Am I grabbed component
      (Default|ReleaseBlock _asplayer_pawn))
    ;[1 1 1] Change Height if not peg
    (if (not (== (Utilities|GetClass OtherComp) "/Game/Blueprint/Blueprints/Hazards/Pegs.Pegs_C"))
      (bind _asplayer_pawn_2 (Utilities|Casting|CastToPlayerPawn (Game|GetPlayerCharacter 0)))
      (Default|ChangeHeight (Variables|/Game/Blueprint/Blueprints/PlayerPawn.PlayerPawn_C|GetBlockCopy _asplayer_pawn_2))
      ;[1 1 1] Play Sound
      (Utilities|FlowControl|Sequence
        (:then_0
          (Utilities|FlowControl|DoOnce false :!label _label
            (:Completed
              (bind _returnvalue_3 (Audio|SpawnSoundatLocation "/Game/Sounds/BlockHits/BlockHit.BlockHit" (.Location (Collision|BreakHitResult Hit)) "0, 0, 0" 1.0 1.0 0.0 0 0))
              (Effects|Components|ParticleSystem|SetIntParameter _returnvalue_3 "Power" (Math|Float|Truncate (Math|Float|MapRangeClamped _returnvalue_2 2e+02 1e+01 0.0 3.0)))
              (Audio|Components|Audio|SetVolumeMultiplier _returnvalue_3 (Math|Float|MapRangeClamped _returnvalue_2 1e+01 0.0 1.0 0.0) :!class /Script/Engine.AudioComponent))))
        (:then_1
          (Utilities|FlowControl|Delay (Math|Random|RandomFloatinRange 0.1 0.3))
          (goto _label Reset))))))

(fn ConstructionScript)