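; Wind hazard actor that pushes released, physics-simulating MoveableBlocks inside a box volume sized from its range variables.
; While anything overlaps the box, Tick fires an evenly spaced X/Z grid of debug-drawn line traces along local +Y.
; Each valid hit applies force at the impact point, with direction and strength derived from the block's right vector and inverted impact normal.
; An unconnected multi-trace loop remains, marked as possibly unneeded.
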(event EventTick
  (params (DeltaSeconds :type Float%20%28single-precision%29))
  (bind _returnvalue (Transformation|GetActorTransform))
  (bind _distbetweentraces (Variables|Default|GetDistBetweenTraces))
  (if (> (Utilities|Array|Length (Class|PrimitiveComponent|GetOverlappingComponents (Variables|Default|GetRange))) 0) ; Is overlapping actors
    ;[1 1 1] Trace Wind Lines
    (for _index (range 0 (Math|Float|Truncate (/ (Variables|Default|GetRangeX) (Variables|Default|GetDistBetweenTraces))))
      (for _index_2 (range 0 (Math|Float|Truncate (/ (Variables|Default|GetRangeZ) (Variables|Default|GetDistBetweenTraces))))
        (bind _outhit (Collision|LineTraceByChannel (Math|Transform|TransformLocation _returnvalue (Math|Vector|MakeVector (- (* _index _distbetweentraces) (/ (Variables|Default|GetRangeX) 2.0)) 0.0 (- (* _index_2 _distbetweentraces) (/ (Variables|Default|GetRangeZ) 2.0)))) (Math|Transform|TransformLocation _returnvalue (+ (Math|Vector|MakeVector (- (* _index _distbetweentraces) (/ (Variables|Default|GetRangeX) 2.0)) 0.0 (- (* _index_2 _distbetweentraces) (/ (Variables|Default|GetRangeZ) 2.0))) (Math|Vector|MakeVector 0.0 (Variables|Default|GetRangeY) 0.0))) "TraceTypeQuery1" true 0 "ForOneFrame"))
        ;[1 1 1] Apply Force
        (if (.bBlockingHit (Collision|BreakHitResult _outhit))
          (bind _asmoveable_block (Utilities|Casting|CastToMoveableBlock (.HitActor (Collision|BreakHitResult _outhit))))
          (if (Variables|/Game/Blueprint/Blueprints/Blocks/MoveableBlock.MoveableBlock_C|GetLetGoOfMe _asmoveable_block)
            (if (Physics|IsSimulatingPhysics (.HitComponent (Collision|BreakHitResult _outhit)) "None")
              (Class|PrimitiveComponent|AddForceatLocation (.HitComponent (Collision|BreakHitResult _outhit)) (* (Math|Vector|Normalize (+ (Transformation|GetActorRightVector (.HitActor (Collision|BreakHitResult _outhit))) (Math|Vector|NegateVector (.ImpactNormal (Collision|BreakHitResult _outhit))))) (* (Math|Float|Absolute(Float) (Math|Vector|DotProduct (Transformation|GetActorRightVector (.HitActor (Collision|BreakHitResult _outhit))) (Math|Vector|NegateVector (.ImpactNormal (Collision|BreakHitResult _outhit))))) (Variables|Default|GetMaxForce))) (.ImpactPoint (Collision|BreakHitResult _outhit)) "None"))))))))

(fn ConstructionScript
  (bind _range (Variables|Default|GetRange))
  (Components|Box|SetBoxExtent (Variables|Default|GetRange) (Math|Vector|MakeVector (/ (Variables|Default|GetRangeX) 2.0) (/ (Variables|Default|GetRangeY) 2.0) (/ (Variables|Default|GetRangeZ) 2.0)) true)
  (Transformation|SetRelativeLocation _range (Math|Vector|MakeVector 0.0 (.y (Variables|/Script/Engine.BoxComponent|GetBoxExtent _range)) 0.0) false false))